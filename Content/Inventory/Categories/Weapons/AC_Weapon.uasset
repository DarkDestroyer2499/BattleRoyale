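; Weapon inventory component that stores owned weapons in a name-keyed map and tracks the active one.
; GiveWeapon looks up the WeaponTable row and adds new weapons to the map.
; For owned weapons, it sets the found struct's Ammo to the table value, without summing or re-adding it to the map.
; CycleUp and CycleDown step through the map keys, update ActiveWeapon and return that weapon's data.
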(fn `CycleDown`
  (returns (Value :type "/Game/Inventory/Categories/Weapons/WeaponStruct Structure"))
  (bind _weapons (`self.Weapons`))
  (bind _keys (`BlueprintMapLibrary.Map_Keys` _weapons))
  (bind _newarrayitem (`/Game/Inventory/ML_Arrays.ML_GetPreviousArrayItem` _keys (`self.ActiveWeapon`)))
  (bind (_value _returnvalue) (`BlueprintMapLibrary.Map_Find` _weapons _newarrayitem))
  (if _returnvalue
    (set `self.ActiveWeapon` _newarrayitem)
    (return _value)
    (else
      (return))))

(fn `CycleUp`
  (returns (Value :type "/Game/Inventory/Categories/Weapons/WeaponStruct Structure"))
  (bind _weapons (`self.Weapons`))
  (bind _keys (`BlueprintMapLibrary.Map_Keys` _weapons))
  (bind _newarrayitem (`/Game/Inventory/ML_Arrays.ML_GetNextArrayItem` _keys (`self.ActiveWeapon`)))
  (bind (_value _returnvalue) (`BlueprintMapLibrary.Map_Find` _weapons _newarrayitem))
  (if _returnvalue
    (set `self.ActiveWeapon` _newarrayitem)
    (return _value)
    (else
      (return))))

(fn `GiveWeapon`
  (params (WeaponName :type Name))
  (bind (_value _returnvalue) (`BlueprintMapLibrary.Map_Find` (`self.Weapons`) (`local.WeaponName`)))
  (`|ExecutionSequence`
    (:`then_0`
      ;[1 1 1] Validate
      (bind _returnvalue_2 (`|GetDataTableRow` "/Game/Inventory/Categories/Weapons/WeaponTable.WeaponTable" (`local.WeaponName`))
        (:`then`
          (set `self.Out Row` _returnvalue_2))
        (:`RowNotFound`
          (set `self.Out Row` (struct))
          (return))))
    (:`then_1`
      ;[1 1 1] Stack weapon
      (if _returnvalue
        (setmembers `/Game/Inventory/Categories/Weapons/WeaponStruct` :`StructRef` _value :`Ammo` (`.Ammo_6_40EA46134314771CCB684BA9CC805BB9` (break `/Game/Inventory/Categories/Weapons/WeaponStruct` (`self.Out Row`))))
        (return)))
    (:`then_2`
      ;[1 1 1] Add Weapon
      (`BlueprintMapLibrary.Map_Add` (`self.Weapons`) (`local.WeaponName`) (`self.Out Row`))
      (return))))