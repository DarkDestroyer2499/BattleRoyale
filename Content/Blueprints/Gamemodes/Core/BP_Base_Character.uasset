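; Base multiplayer character with movement, sprinting, crouching, aiming, firing and parachuting.
; Input calls paired server/client events to set states, with timelines easing aim camera distance and crouch capsule height.
; ACWeapon supplies cycled weapons, soft-loaded into a hand-socket child actor with an animation overlay state; firing, allowed while aiming, messages that actor.
; Holding jump high above ground enables parachuting, whose OnRep toggles the mesh and clamps fall speed upon opening.
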(event `self.ReceiveBeginPlay`
  (bind _returnvalue (`|CreateWidget` "/Game/WeaponSystem/UI_Crosshair.UI_Crosshair_C"))
  (set `self.Crosshair` _returnvalue)
  (set `self.DefaultCamDistance` (`SpringArmComponent.TargetArmLength` (`self.SpringArm`))))

(event `InputAxis|Move Forward / backward`
  (params (AxisValue :type "Float (single-precision)"))
  ;[1 1 1] Movement
  (`self.AddMovementInput` (`self.GetActorForwardVector`) AxisValue))

(event `InputAxis|move Right / Left`
  (params (AxisValue :type "Float (single-precision)"))
  ;[1 1 1] Movement
  (`self.AddMovementInput` (`self.GetActorRightVector`) AxisValue))

(event `InputAxis|Look UP / Down Mouse`
  (params (AxisValue :type "Float (single-precision)"))
  ;[1 1 1] Looking
  (`self.AddControllerPitchInput` AxisValue))

(event `self.ReceiveTick`
  (params (DeltaSeconds :type "Float (single-precision)"))
  ;[1 1 1] Parachuting Logic
  (if (`self.WantsToParachute?`)
    (set `self.IsParachuting?` (`self.CanUseParachute?`))
    (elif (`self.IsParachuting?`)
      (set `self.IsParachuting?` false))))

(event `InputAxis|Turn Right / Left Mouse`
  (params (AxisValue :type "Float (single-precision)"))
  ;[1 1 1] Looking
  (`self.AddControllerYawInput` AxisValue))

(event `SR_Set_WantsToParachute?`
  (params (`WantsToParachute?` :type Boolean))
  ;[1 1 1] Server : Set Wants To Parachute
  (set `self.WantsToParachute?` `WantsToParachute?`))

(event `InputAction|Jumping`
  (params (Key :type "Key Structure"))
  ;[1 1 1] Jumping
  (:`Pressed`
    (`self.Jump`)
    (bind _output_get (set `self.WantsToParachute?` true))
    (`self.SR_Set_WantsToParachute?` _output_get))
  (:`Released`
    (`self.StopJumping`)
    (set `self.WantsToParachute?` false)
    (`self.SR_Set_WantsToParachute?` false)))

(event `Key|LeftShift`
  (params (Key :type "Key Structure"))
  ;[1 1 1] Sprinting
  (:`Pressed`
    (`self.Sprint On Server`)
    (`self.Sprint ON Client`)
    (if (`self.Crouching`)
      (`self.Crouch OFF Server`)
      (`self.Crouch OFF Client`)
      (`self.Crouch Cam OFF Server`)))
  (:`Released`
    (`self.Sprint OFF Server`)
    (`self.Sprint OFF Client`)))

(event `Key|LeftControl`
  (params (Key :type "Key Structure"))
  ;[1 1 1] Crouch
  (:`Pressed`
    (`self.Crouch ON Server`)
    (`self.Crouch ON Client`)
    (`self.Sprint OFF Server`)
    (`self.Sprint OFF Client`)
    (`self.Crouch Cam On Server`))
  (:`Released`
    (`self.Crouch OFF Server`)
    (`self.Crouch OFF Client`)
    (`self.Crouch Cam OFF Server`)))

(event `Key|RightMouseButton`
  (params (Key :type "Key Structure"))
  (bind _crosshair (`self.Crosshair`))
  ;[1 1 1] Aim
  (:`Pressed`
    (`UserWidget.AddToViewport` _crosshair 0)
    (`self.Aim Cam ON Server`)
    (`self.Aim ON Server`)
    (`self.Aim ON Client`))
  (:`Released`
    (`Widget.RemoveFromParent` _crosshair)
    (`self.Aim Cam OFF Server`)
    (`self.Aim OFF Server`)
    (`self.Aim OFF Client`)))

(event `Key|MouseScrollUp`
  (params (Key :type "Key Structure"))
  ;[1 1 1] Weapon Cycle
  (:`Pressed`
    (`self.CycleUp Server`)))

(event `Key|MouseScrollDown`
  (params (Key :type "Key Structure"))
  ;[1 1 1] Weapon Cycle
  (:`Pressed`
    (`self.CycleDown Server`)))

(event `Key|LeftMouseButton`
  (params (Key :type "Key Structure"))
  ;[1 1 1] Fire Weapon
  (:`Pressed`
    (if (`self.Aiming`)
      (`self.Fire Server` true)))
  (:`Released`
    (`self.Fire Server` false)))

(event `self.ReceiveAnyDamage`
  (params (Damage :type "Float (single-precision)") (DamageType :type "DamageType Object Reference") (InstigatedBy :type "Controller Object Reference") (DamageCauser :type "Actor Object Reference"))
  (`KismetSystemLibrary.PrintString` "Damage" true true (struct :`R` 1.0 :`B` 0.735957 :`A` 1.0)))

(event `Fire Milti`
  (params (CanFire :type Boolean))
  (bind _childactor (`ChildActorComponent.ChildActor` (`self.HandObject`)))
  ;[1 1 1] Fire Weapon
  (if CanFire
    (message `/Game/WeaponSystem/BPI_Weapon.FireON` _childactor)
    (else
      (message `/Game/WeaponSystem/BPI_Weapon.FireOFF` _childactor))))

(event `Aim Cam ON Client`
  (bind _defaultcamdistance (`self.DefaultCamDistance`))
  ;[1 1 1] Aim Cam
  (bind (_direction _alpha) (`Timeline|Aim Cam` :!label _label)
    (:`Update`
      (set `SpringArmComponent.TargetArmLength` (`KismetMathLibrary.Lerp` _defaultcamdistance (/ _defaultcamdistance (`self.AimingCamDistanceDivider`)) _alpha) (`self.SpringArm`)))))

(event `Crouch ON Client`
  ;[1 1 1] Crouch
  (set `self.Crouching` true))

(event `Aim Cam OFF Client`
  ;[1 1 1] Aim Cam
  (goto _label :!via `ReverseFromEnd`))

(event `Sprint ON Client`
  ;[1 1 1] Sprint
  (`self.SetSprint` true))

(event `Fire Server`
  (params (CanFire :type Boolean))
  ;[1 1 1] Fire Weapon
  (`self.Fire Milti` CanFire))

(event `Crouch ON Server`
  ;[1 1 1] Crouch
  (set `self.Crouching` true))

(event `Sprint On Server`
  ;[1 1 1] Sprint
  (`self.SetSprint` true))

(event `Aim Cam ON Server`
  ;[1 1 1] Aim Cam
  (`self.Aim Cam ON Client`))

(event `Crouch OFF Client`
  ;[1 1 1] Crouch
  (set `self.Crouching` false))

(event `Aim Cam OFF Server`
  ;[1 1 1] Aim Cam
  (`self.Aim Cam Off Client`))

(event `Sprint OFF Client`
  ;[1 1 1] Sprint
  (`self.SetSprint` false))

(event `Crouch OFF Server`
  ;[1 1 1] Crouch
  (set `self.Crouching` false))

(event `Sprint OFF Server`
  ;[1 1 1] Sprint
  (`self.SetSprint` false))

(event `Crouch Cam ON Client`
  ;[1 1 1] Crouch Cam
  (bind (_direction _alpha) (`Timeline|Crouch Cam` :!label _label_2)
    (:`Update`
      (`CapsuleComponent.SetCapsuleHalfHeight` (`self.CapsuleComponent`) (`KismetMathLibrary.Lerp` 88.0 68.0 _alpha) true))))

(event `Set Overlay Client`
  (params (OverlayState :type "/Game/Characters/Mannequins/Animations/Manny/Unarmed/OverlayStates Enum" :default "NewEnumerator0"))
  ;[1 1 1] Overlay State
  (set `self.OverlayState` OverlayState))

(event `Crouch Cam OFF Client`
  ;[1 1 1] Crouch Cam
  (goto _label_2 :!via `ReverseFromEnd`))

(event `Set Overlay Server`
  (params (OverlayState :type "/Game/Characters/Mannequins/Animations/Manny/Unarmed/OverlayStates Enum" :default "NewEnumerator0"))
  ;[1 1 1] Overlay State
  (set `self.OverlayState` OverlayState))

(event `Crouch Cam On Server`
  ;[1 1 1] Crouch Cam
  (`self.Crouch Cam ON Client`))

(event `Crouch Cam OFF Server`
  ;[1 1 1] Crouch Cam
  (`self.Crouch Cam OFF Client`))

(event `Aim ON Client`
  ;[1 1 1] Aiming
  (set `self.Aiming` true))

(event `CycleUp Multi`
  ;[1 1 1] Cycle Weapon
  (bind _value (`/Game/Inventory/Categories/Weapons/AC_Weapon.CycleUp` (`self.AC_Weapon`)))
  (bind (_mesh _ammo _overlay _actor_bp _sockettransform) (break `/Game/Inventory/Categories/Weapons/WeaponStruct` _value))
  (`self.AttachToHand` _overlay _actor_bp _sockettransform))

(event `Aim ON Server`
  ;[1 1 1] Aiming
  (set `self.Aiming` true))

(event `Aim OFF Client`
  ;[1 1 1] Aiming
  (set `self.Aiming` false))

(event `CycleUp Server`
  ;[1 1 1] Cycle Weapon
  (`self.CycleUp Multi`))

(event `Aim OFF Server`
  ;[1 1 1] Aiming
  (set `self.Aiming` false))

(event `CycleDown Multi`
  ;[1 1 1] Cycle Weapon
  (bind _value (`/Game/Inventory/Categories/Weapons/AC_Weapon.CycleDown` (`self.AC_Weapon`)))
  (bind (_mesh _ammo _overlay _actor_bp _sockettransform) (break `/Game/Inventory/Categories/Weapons/WeaponStruct` _value))
  (`self.AttachToHand` _overlay _actor_bp _sockettransform))

(event `CycleDown Server`
  ;[1 1 1] Cycle Weapon
  (`self.CycleDown Multi`))

(fn `AttachToHand`
  (params (Overlay :type "/Game/Characters/Mannequins/Animations/Manny/Unarmed/OverlayStates Enum" :default "NewEnumerator0") (`Actor BP` :type "Actor Soft Class Reference") (`Socket Transform` :type "Transform Structure"))
  (bind _handobject (`self.HandObject`))
  (bind _overlay (`local.Overlay`))
  (if (`KismetSystemLibrary.IsValidSoftClassReference` `Actor BP`)
    (bind _returnvalue (`KismetSystemLibrary.LoadClassAsset_Blocking` `Actor BP`))
    (bind _asactor (castclass `Actor` _returnvalue))
    (`ChildActorComponent.SetChildActorClass` _handobject _asactor)
    (`SceneComponent.K2_AttachToComponent` _handobject (`self.Mesh`) "hand_r" "SnapToTarget" "SnapToTarget" "SnapToTarget" true)
    (`SceneComponent.K2_SetRelativeTransform` (`self.HandObject`) (`local.Socket Transform`) true true)
    (else
      (`ChildActorComponent.SetChildActorClass` (`self.HandObject`) null)))
  (`self.Set Overlay Server` _overlay)
  (`self.Set Overlay Client` _overlay)
  (return))

(fn `CanUseParachute?`
  (returns (`CanParachute?` :type Boolean))
  (bind (_returnvalue_x _returnvalue_y _returnvalue_z) (`KismetMathLibrary.BreakVector` (`self.K2_GetActorLocation`)))
  (return (>= (- _returnvalue_z (.z (`.Location` (`GameplayStatics.BreakHitResult` (`.HitResult` (break `FindFloorResult` (`CharacterMovementComponent.K2_FindFloor` (`self.CharacterMovement`) (`self.K2_GetActorLocation`)))))))) 1000.0)))

(fn `GetCamera`
  (returns (WorldLocation :type "Vector Structure") (ForwardVector :type "Vector Structure"))
  (bind _camera (`self.Camera`))
  (return (`SceneComponent.K2_GetComponentLocation` _camera) (`SceneComponent.GetForwardVector` _camera)))

(fn `GetWeaponName`
  (returns (WeaponName :type Name))
  (return (`/Game/Inventory/Categories/Weapons/AC_Weapon.ActiveWeapon` (`self.AC_Weapon`))))

(fn `OnRep_IsParachuting?`
  (bind (_returnvalue_x _returnvalue_y _returnvalue_z) (`KismetMathLibrary.BreakVector` (`self.GetVelocity`)))
  (bind (_returnvalue_x_2 _returnvalue_y_2 _returnvalue_z_2) (`KismetMathLibrary.BreakVector` (`self.GetVelocity`)))
  (`SceneComponent.SetVisibility` (`self.SM_Parachute`) (`self.IsParachuting?`) false)
  (if (`self.IsParachuting?`)
    (if (<= _returnvalue_z_2 -750.0)
      (set `MovementComponent.Velocity` (`KismetMathLibrary.MakeVector` _returnvalue_x _returnvalue_y (`KismetMathLibrary.FClamp` _returnvalue_z -750.0 0.0)) (`self.CharacterMovement`)))))

(fn `PickupWeapon`
  (params (WeaponName :type Name))
  (returns (Success :type Boolean))
  (`/Game/Inventory/Categories/Weapons/AC_Weapon.GiveWeapon` (`self.AC_Weapon`) WeaponName)
  (`KismetSystemLibrary.PrintString` (`KismetStringLibrary.Conv_NameToString` WeaponName))
  (bind _value (`/Game/Inventory/Categories/Weapons/AC_Weapon.CycleUp` (`self.AC_Weapon`)))
  (bind (_mesh _ammo _overlay _actor_bp _sockettransform) (break `/Game/Inventory/Categories/Weapons/WeaponStruct` _value))
  (`self.AttachToHand` _overlay _actor_bp _sockettransform)
  (return true))

(fn `SetSprint`
  (params (Enable :type Boolean))
  (bind _charactermovement (`self.CharacterMovement`))
  (if Enable
    (set `self.Sprinting` true)
    (set `CharacterMovementComponent.MaxWalkSpeed` 525.0 _charactermovement)
    (else
      (set `self.Sprinting` false)
      (set `CharacterMovementComponent.MaxWalkSpeed` 310.0 _charactermovement))))

(fn `UserConstructionScript`)