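; Core player controller that starts in game-only input and toggles the in-game menu from an input action.
; ToogleGameMenu creates WB_GameMenu on first use, caches it, and afterwards switches it between visible and collapsed.
; FocusWidget shows the cursor with game-and-UI input, then returns focus to the game viewport, while FocusGame hides the cursor and restores game-only input.
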(event `self.ReceiveBeginPlay`
  (`WidgetBlueprintLibrary.SetInputMode_GameOnly` self))

(event `InputAction|ToogleGameMenu`
  (params (Key :type "Key Structure"))
  (:`Pressed`
    (`self.ToogleGameMenu`)))

(fn `Focus Widget`
  (params (PlayerController :type "PlayerController Object Reference"))
  (set `self.bShowMouseCursor` true)
  (`WidgetBlueprintLibrary.SetInputMode_GameAndUIEx` (`GameplayStatics.GetPlayerController` 0) (`self.WB_GameMenu`))
  (`WidgetBlueprintLibrary.SetFocusToGameViewport`))

(fn `FocusGame`
  (returns (ReturnValue :type "PlayerController Object Reference"))
  (bind _returnvalue (`GameplayStatics.GetPlayerController` 0))
  (set `self.bShowMouseCursor` false)
  (`WidgetBlueprintLibrary.SetInputMode_GameOnly` _returnvalue)
  (return _returnvalue))

(fn `ToogleGameMenu`
  (bind _wb_gamemenu (`self.WB_GameMenu`))
  (`self.WB_GameMenu`
    (:`then`
      (if (`Widget.IsVisible` _wb_gamemenu)
        (`Widget.SetVisibility` _wb_gamemenu "Collapsed")
        (`self.FocusGame`)
        (else
          (`Widget.SetVisibility` _wb_gamemenu "Visible")
          (`self.Focus Widget` null :!label _label))))
    (:`else`
      (bind _returnvalue (`|CreateWidget` "/Game/Wigets/GameWidgets/WB_GameMenu.WB_GameMenu_C" self))
      (bind _output_get (set `self.WB_GameMenu` _returnvalue))
      (`UserWidget.AddToViewport` _output_get 0)
      (goto _label))))

(fn `UserConstructionScript`)