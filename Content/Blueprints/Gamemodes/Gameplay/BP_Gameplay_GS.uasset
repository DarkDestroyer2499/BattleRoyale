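; Game state for gameplay that starts a pre-match countdown once enough players have connected.
; A connection notification updates the player count and, at the required minimum, sets the countdown a single time.
; The countdown's RepNotify refreshes every match-start countdown widget and, on authority, re-triggers a one-second delayed decrement, forming a self-driving timer.
; At zero it only prints that the match has started.
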(event `/Game/Blueprints/Interfaces/BPI_GameState.Notify_PlayerConnection`
  (bind _returnvalue (`GameplayStatics.GetNumPlayerStates`))
  (`KismetSystemLibrary.PrintString` "Player Connected")
  (set `self.CurrentAmountOfPlayers` _returnvalue)
  (if (>= _returnvalue (`self.MinimumRequiredPlayers`))
    (`/Engine/EditorBlueprintResources/StandardMacros.DoOnce` false
      (:`Completed`
        (set `self.MatchStart_CountDown` 15)))))

(event `Match_CountDown`
  (`KismetSystemLibrary.Delay` 1.0)
  (set `self.MatchStart_CountDown` (- (`self.MatchStart_CountDown`) 1)))

(fn `OnRep_MatchStart_CountDown`
  (`self.Update_matchStartCountdownWidget`)
  (`/Engine/EditorBlueprintResources/ActorMacros.Switch Has Authority`
    (:`Authority`
      (if (== (`self.MatchStart_CountDown`) 15)
        (`self.Match_CountDown`)
        (elif (== (`self.MatchStart_CountDown`) 0)
          (`KismetSystemLibrary.PrintString` "Started Match" true true (struct :`R` 0.014836 :`G` 1.0 :`A` 1.0) 15.0)
          (else
            (`self.Match_CountDown`)))))))

(fn `Update_matchStartCountdownWidget`
  (bind _foundwidgets (`WidgetBlueprintLibrary.GetAllWidgetsOfClass` "/Game/Wigets/GameWidgets/WB_MatchStartCountdown.WB_MatchStartCountdown_C" false))
  (for _array_element _foundwidgets
    (`/Game/Wigets/GameWidgets/WB_MatchStartCountdown.Update_Widget` _array_element (`self.MatchStart_CountDown`))))

(fn `UserConstructionScript`
  (`parent.UserConstructionScript`))