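; BP_Gameplay_PC is a gameplay player controller that puts the gameplay HUD on screen for the local player.
; On BeginPlay, after the parent logic, it checks that it is a local controller, then creates WB_GamePlay_HUD owned by itself, stores it in WBHUD and adds it to the viewport.
; Tick is disabled and the construction script only calls its parent.
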(event `self.ReceiveBeginPlay`
  (`parent.ReceiveBeginPlay`)
  (if (`self.IsLocalPlayerController`)
    (bind _returnvalue (`|CreateWidget` "/Game/Wigets/GameWidgets/WB_GamePlay_HUD.WB_GamePlay_HUD_C" self))
    (bind _output_get (set `self.WB HUD` _returnvalue))
    (`UserWidget.AddToViewport` _output_get 0)))

(fn `UserConstructionScript`
  (`parent.UserConstructionScript`))