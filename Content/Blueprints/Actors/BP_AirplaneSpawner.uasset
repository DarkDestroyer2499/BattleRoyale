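; BP_AirplaneSpawner is an actor that spawns a BP_Airplane from a random direction, on authority only, whenever SpawnAirplane is called.
; It randomizes its own yaw, then spawns the plane at its Arrow component, aimed toward the actor's location with a -90 degree yaw offset.
; After spawning, it sets the SpringArm length to half the new plane's FinishDistance.
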(event `SpawnAirplane`
  (bind _returnvalue (`SceneComponent.K2_GetComponentLocation` (`self.Arrow`)))
  (bind (_returnvalue_roll _returnvalue_pitch _returnvalue_yaw) (`KismetMathLibrary.BreakRotator` (`KismetMathLibrary.FindLookAtRotation` _returnvalue (`self.K2_GetActorLocation`))))
  (`/Engine/EditorBlueprintResources/ActorMacros.Switch Has Authority`
    (:`Authority`
      (`self.K2_SetActorRotation` (`KismetMathLibrary.MakeRotator` 0.0 0.0 (`KismetMathLibrary.RandomFloatInRange` 0.0 360.0)))
      (bind _returnvalue_2 (`|SpawnActorFromClass` "/Game/Blueprints/Actors/BP_Airplane.BP_Airplane_C" (`KismetMathLibrary.MakeTransform` _returnvalue (`KismetMathLibrary.MakeRotator` _returnvalue_roll _returnvalue_pitch (- _returnvalue_yaw 90.0))) "Undefined" "MultiplyWithRoot" null null))
      (set `SpringArmComponent.TargetArmLength` (`KismetMathLibrary.Conv_Int64ToDouble` (/ (`/Game/Blueprints/Actors/BP_Airplane.FinishDistance` _returnvalue_2) 2)) (`self.SpringArm`)))))

(fn `UserConstructionScript`)