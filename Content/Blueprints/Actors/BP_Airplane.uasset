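; BP_Airplane is a plane actor that carries gameplay characters along a straight or gravity-affected flight path.
; On BeginPlay the server configures ProjectileMovement from its speed, gravity and velocity variables, then teleports every BP_Gameplay_Character to random points inside its Box component.
; On Tick the server prints the distance from the start location and destroys the plane once it reaches FinishDistance.
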(event `self.ReceiveBeginPlay`
  (bind _projectilemovement (`self.ProjectileMovement`))
  (bind _projectile_speed (`self.Projectile speed`))
  ;[1 1 1] Plane's location, gravity, speed
  (`/Engine/EditorBlueprintResources/ActorMacros.Switch Has Authority`
    (:`Authority`
      (set `self.StartLocation` (`self.K2_GetActorLocation`))
      (set `ProjectileMovementComponent.InitialSpeed` _projectile_speed _projectilemovement)
      (set `ProjectileMovementComponent.MaxSpeed` _projectile_speed _projectilemovement)
      (set `ProjectileMovementComponent.ProjectileGravityScale` (`self.Projectile gravity scale`) _projectilemovement)
      (`ProjectileMovementComponent.SetVelocityInLocalSpace` _projectilemovement (`self.Velocity Vector`))
      ;[1 1 1] Spawn Players inside Plane
      (`self.SpawnPlayersInPlane`))))

(event `self.ReceiveTick`
  (params (DeltaSeconds :type "Float (single-precision)"))
  (bind _returnvalue (`KismetMathLibrary.Vector_Distance` (`self.StartLocation`) (`self.K2_GetActorLocation`)))
  ;[1 1 1] Destroy plane after distance
  (`/Engine/EditorBlueprintResources/ActorMacros.Switch Has Authority`
    (:`Authority`
      (`KismetSystemLibrary.PrintString` (`KismetStringLibrary.Conv_DoubleToString` _returnvalue))
      (if (>= _returnvalue (`self.FinishDistance`))
        (`self.K2_DestroyActor`)))))

(fn `SpawnPlayersInPlane`
  (bind _outactors (`GameplayStatics.GetAllActorsOfClass` "/Game/Blueprints/Gamemodes/Gameplay/BP_Gameplay_Character.BP_Gameplay_Character_C"))
  (for _array_element _outactors
    (`self.K2_SetActorLocation` _array_element (`KismetMathLibrary.RandomPointInBoundingBox` (`SceneComponent.K2_GetComponentLocation` (`self.Box`)) (32.0 32.0 32.0)) false true)))

(fn `UserConstructionScript`)